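; SkiManGameMode sets up local multiplayer for the ski game and handles pawn swapping.
; BeginPlay caches PlayerStarts and creates players in a NumberOfPlayers counter loop.
; SpawnCharacter and DespawnPlayer destroy the controlled pawn, then spawn and possess a BP_SkiMan or InitPawn respectively.
; Both use GetRandomSpawn, whose random PlayerStart lookup appears unconnected; GameCamera view blends are also unwired.
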(event Custom|SpawnCharacter
  (params (PlayerController :type Ski%20Man%20Controller%20Object%20Reference))
  (bind _returnvalue (Pawn|GetControlledPawn PlayerController))
  (Utilities|IsValid _returnvalue
    (:Is%20Valid
      (Actor|DestroyActor _returnvalue)
      (bind _returnvalue_2 (Game|SpawnActorfromClass "/Game/Blueprints/BP_SkiMan.BP_SkiMan_C" (Utilities|GetRandomSpawn) "Undefined" _returnvalue 0))
      (Pawn|Possess PlayerController _returnvalue_2))))

(event Custom|DespawnPlayer
  (params (PlayerController :type Ski%20Man%20Controller%20Object%20Reference))
  (bind _returnvalue (Pawn|GetControlledPawn PlayerController))
  (Utilities|IsValid _returnvalue
    (:Is%20Valid
      (Actor|DestroyActor _returnvalue)
      (bind _returnvalue_2 (Game|SpawnActorfromClass "/Game/Blueprints/InitPawn.InitPawn_C" (Utilities|GetRandomSpawn) "Undefined" _returnvalue 0))
      (Pawn|Possess PlayerController _returnvalue_2))))

(event EventBeginPlay
  (bind _outactors (Actor|GetAllActorsOfClass "/Script/Engine.PlayerStart"))
  (Variables|Default|SetSpawnPoints _outactors)
  (while (<= (Variables|Default|GetNumberOfPlayers) 2)
    (bind _result (Math|Integer|IncrementInt (Variables|Default|GetNumberOfPlayers))
      (:%20%20
        (Variables|Default|SetNumberOfPlayers _result)
        (Class|GameplayStatics|CreatePlayer -1)))))

(fn ConstructionScript)