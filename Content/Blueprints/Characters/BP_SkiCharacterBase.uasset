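; Base ski character Blueprint that smooths the mesh's movement on non-authority clients and toggles capsule visibility with the C key.
; Shortly after BeginPlay, clients reparent the mesh to a detached RotationCorrection component.
; Each client tick, RotationCorrection lerps toward the capsule's rotation and the TargetLocation component's position.
; TargetLocation slides forward with smoothed per-update travel distance, offsetting the interpolation lag at speed.
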(event EventTick
  (params (DeltaSeconds :type Float%20%28single-precision%29))
  (|CallParentFunction DeltaSeconds)
  (Networking|SwitchHasAuthority
    (:Remote
      (CallFunction|UpdateRawandSmoothSpeed)
      (CallFunction|UpdatedTargetLocation)
      (Transformation|SetWorldLocation (Variables|Default|GetRotationCorrection) (Math|Vector|Lerp(Vector) (Transformation|GetWorldLocation (Variables|Default|GetRotationCorrection)) (Transformation|GetWorldLocation (Variables|Default|GetTargetLocation)) 0.09) false false)
      (Transformation|SetWorldRotation (Variables|Default|GetRotationCorrection) (Math|Rotator|Lerp(Rotator) (Transformation|GetWorldRotation (Variables|Default|GetRotationCorrection)) (Transformation|GetWorldRotation (Variables|Default|GetCapsuleComponent)) 0.1 true) false false))))

(event EventBeginPlay
  (bind _mesh (Variables|Character|GetMesh))
  (|CallParentFunction)
  (Utilities|FlowControl|Delay 0.2)
  (Networking|SwitchHasAuthority
    (:Remote
      (Transformation|DetachFromComponent (Variables|Character|GetMesh) "KeepWorld" "KeepWorld" "KeepWorld" true)
      (Transformation|DetachFromComponent (Variables|Default|GetRotationCorrection) "KeepWorld" "KeepWorld" "KeepWorld" true)
      (Transformation|AttachComponentToComponent _mesh (Variables|Default|GetRotationCorrection) "None" "SnapToTarget" "SnapToTarget" "KeepWorld" true)
      (Transformation|SetWorldRotation _mesh "0,-90.000000, 0" false false))))

(event Input|KeyboardEvents|C
  (params (Key :type Key%20Structure :default "None"))
  (:Pressed
    (bind _isa (Utilities|FlowControl|FlipFlop)
      (:A
        _)
      (:B
        _))
    (Development|SetHiddeninGame (Variables|Default|GetCapsuleComponent) _isa false)))

(fn ConstructionScript)

(fn UpdateRawandSmoothSpeed
  (bind _returnvalue (Transformation|GetActorLocation))
  (if (Math|Vector|NotEqual(Vector) (Transformation|GetActorLocation) (Variables|Default|GetLastLocation) 0.0001)
    (Variables|Default|SetCurrentRawSpeed (Math|Vector|VectorLength (- _returnvalue (Variables|Default|GetLastLocation))))
    (Variables|Default|SetLastLocation _returnvalue))
  (Variables|Default|SetCurrentSmoothedSpeed (Math|Float|Lerp (Variables|Default|GetCurrentSmoothedSpeed) (Variables|Default|GetCurrentRawSpeed) 0.02)))

(fn UpdatedTargetLocation
  (Transformation|SetRelativeLocation (Variables|Default|GetTargetLocation) (Math|Vector|Lerp(Vector) "0.000000, 0,-60.000000" "300.000000, 0,-60.000000" (Math|Float|NormalizetoRange (Variables|Default|GetCurrentSmoothedSpeed) 0.0 6e+01)) false false))