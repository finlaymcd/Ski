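; Player skier driven by physics forces on its capsule, with keys for turning, tucking and a push animation.
; Each tick feeds input to the anim blueprint, eases the camera behind it and traces for ground.
; Grounded, the anim turn value drives curve-scaled sideways force and rotation follows travel direction; airborne, left/right apply spin torque.
; A velocity-aligned force, stronger when tucked, plus constant downward force apply throughout.
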(event EventTick
  (params (DeltaSeconds :type Float%20%28single-precision%29))
  (bind _box (Variables|Default|GetBox))
  (bind _capsulecomponent (Variables|Collision|GetCapsuleComponent))
  (bind _returnvalue (Transformation|GetComponentVelocity _capsulecomponent))
  (bind _returnvalue_2 (Transformation|GetWorldLocation _box))
  (CallFunction|HandleAnims)
  (CallFunction|HandleCameraPos)
  (bind _returnvalue_3 (Collision|LineTraceForObjects _returnvalue_2 (- _returnvalue_2 (* (Math|Vector|GetUpVector _box) 1e+02)) (Utilities|Array|MakeArray "ObjectTypeQuery1") false (Utilities|Array|MakeArray self) "None"))
  (Variables|Default|SetTouchingGround _returnvalue_3)
  (if _returnvalue_3
    (CallFunction|HandleTurning)
    (CallFunction|LerpRotationtoVelocity)
    (else
      (CallFunction|HandleAerial)))
  (Physics|AddForce _capsulecomponent (+ (* (Math|Vector|Normalize _returnvalue) (* (select (Variables|Default|GetDownPressed) 1e+01 5.0) (Math|Vector|VectorLength _returnvalue))) "0, 0,-50000.000000") "None" false))

(event EventBeginPlay
  (Variables|Default|SetABP (.AsABPSki%20Man (Utilities|Casting|CastToABPSkiMan (Components|SkeletalMesh|GetAnimInstance (Variables|Character|GetMesh)))))
  (Variables|Default|SetPreviousLocation (Transformation|GetActorLocation))
  (Variables|Default|SetPreviousCamPos (Transformation|GetWorldLocation (Variables|Default|GetCamera)))
  (Variables|Default|SetPreviousRotation (Transformation|GetActorRotation)))

(event Input|KeyboardEvents|Left
  (params (Key :type Key%20Structure))
  (:Pressed
    (Variables|Default|SetLeftPressed true))
  (:Released
    (Variables|Default|SetLeftPressed false)))

(event Input|KeyboardEvents|Right
  (params (Key :type Key%20Structure))
  (:Pressed
    (Variables|Default|SetRightPressed true))
  (:Released
    (Variables|Default|SetRightPressed false)))

(event Input|KeyboardEvents|Down
  (params (Key :type Key%20Structure))
  (:Pressed
    (Variables|Default|SetDownPressed true))
  (:Released
    (Variables|Default|SetDownPressed false)))

(event Input|KeyboardEvents|SpaceBar
  (params (Key :type Key%20Structure))
  (:Pressed
    (Variables|Default|SetPushPressed true))
  (:Released
    (Variables|Default|SetPushPressed false)))

(fn ConstructionScript)

(fn HandleAnims
  (bind _abp (Variables|Default|GetABP))
  (bind _abp_2 (Variables|Default|GetABP))
  (bind _abp_3 (Variables|Default|GetABP))
  (bind _abp_4 (Variables|Default|GetABP))
  (bind _abp_5 (Variables|Default|GetABP))
  (if (Variables|Default|GetLeftPressed)
    (LocalVariables|SetTurnKeyPressed true)
    (Variables|/Game/SkiMan/ABPSkiMan.ABPSkiMan_C|SetTurnValue _abp_4 (+ (Variables|/Game/SkiMan/ABPSkiMan.ABPSkiMan_C|GetTurnValue _abp_4) (* (Variables|Default|GetTurnSpeed) (Utilities|Time|GetWorldDeltaSeconds)))))
  (if (Variables|Default|GetRightPressed)
    (LocalVariables|SetTurnKeyPressed true)
    (Variables|/Game/SkiMan/ABPSkiMan.ABPSkiMan_C|SetTurnValue _abp (- (Variables|/Game/SkiMan/ABPSkiMan.ABPSkiMan_C|GetTurnValue _abp) (* (Variables|Default|GetTurnSpeed) (Utilities|Time|GetWorldDeltaSeconds)))))
  (if (LocalVariables|GetTurnKeyPressed)
    _
    (else
      (CallFunction|MoveTurntoIdle)))
  (if (Variables|Default|GetDownPressed)
    (Variables|/Game/SkiMan/ABPSkiMan.ABPSkiMan_C|SetTuckValue _abp_3 (Math|Float|Clamp(Float) (- (Variables|/Game/SkiMan/ABPSkiMan.ABPSkiMan_C|GetTuckValue _abp_3) (* (Variables|Default|GetTuckSpeed) (Utilities|Time|GetWorldDeltaSeconds))) 0.0 1e+02))
    (else
      (Variables|/Game/SkiMan/ABPSkiMan.ABPSkiMan_C|SetTuckValue _abp_5 (Math|Float|Clamp(Float) (+ (Variables|/Game/SkiMan/ABPSkiMan.ABPSkiMan_C|GetTuckValue _abp_5) (* (Variables|Default|GetTuckSpeed) (Utilities|Time|GetWorldDeltaSeconds))) 0.0 1e+02))))
  (Variables|/Game/SkiMan/ABPSkiMan.ABPSkiMan_C|SetTurnValue _abp_2 (Math|Float|Clamp(Float) (Variables|/Game/SkiMan/ABPSkiMan.ABPSkiMan_C|GetTurnValue _abp_2) 0.0 1e+02))
  (Variables|/Game/SkiMan/ABPSkiMan.ABPSkiMan_C|SetPushing (Variables|Default|GetABP) (Variables|Default|GetPushPressed)))

(fn MoveTurntoIdle
  (bind _returnvalue (Utilities|Time|GetWorldDeltaSeconds))
  (bind _turnspeed (Variables|Default|GetTurnSpeed))
  (bind _abp (Variables|Default|GetABP))
  (bind _returnvalue_2 (* _turnspeed _returnvalue))
  (if (not (Math|Float|NearlyEqual(Float) (Variables|/Game/SkiMan/ABPSkiMan.ABPSkiMan_C|GetTurnValue (Variables|Default|GetABP)) 5e+01 4.0))
    (if (> (Variables|/Game/SkiMan/ABPSkiMan.ABPSkiMan_C|GetTurnValue (Variables|Default|GetABP)) 5e+01)
      (Variables|/Game/SkiMan/ABPSkiMan.ABPSkiMan_C|SetTurnValue _abp (- (Variables|/Game/SkiMan/ABPSkiMan.ABPSkiMan_C|GetTurnValue (Variables|Default|GetABP)) _returnvalue_2))
      (else
        (Variables|/Game/SkiMan/ABPSkiMan.ABPSkiMan_C|SetTurnValue _abp (+ (Variables|/Game/SkiMan/ABPSkiMan.ABPSkiMan_C|GetTurnValue (Variables|Default|GetABP)) _returnvalue_2))))))

(fn HandleTurning
  (bind _capsulecomponent (Variables|Collision|GetCapsuleComponent))
  (bind _abp (Variables|Default|GetABP))
  (bind _returnvalue (Transformation|GetComponentVelocity _capsulecomponent))
  (bind _turnvalue (Variables|/Game/SkiMan/ABPSkiMan.ABPSkiMan_C|GetTurnValue _abp))
  (if (not (Math|Float|NearlyEqual(Float) _turnvalue 5e+01 1.0))
    (Physics|AddForce (Variables|Collision|GetCapsuleComponent) (* (* (Math|Vector|RotateVectorAroundAxis (Math|Vector|Normalize _returnvalue) -9e+01 "0,0.000000,1.000000") (- _turnvalue 5e+01)) (Math|Curves|GetFloatValue (Variables|Default|GetVelocityTurnCurve) (Math|Vector|VectorLength _returnvalue))) "None" false)))

(fn HandleCameraPos
  (bind _camera (Variables|Default|GetCamera))
  (Transformation|SetWorldLocation _camera (Math|Vector|Lerp(Vector) (Transformation|GetWorldLocation (Variables|Default|GetCamera)) (Transformation|GetWorldLocation (Variables|Default|GetCameraTarget)) 0.1) false false)
  (Transformation|SetWorldRotation _camera (Math|Rotator|FindLookatRotation (Transformation|GetWorldLocation (Variables|Default|GetCamera)) (Transformation|GetWorldLocation (Variables|Default|GetCameraLookatTarget))) false false))

(fn LerpRotationtoVelocity
  (Transformation|SetActorRotation (Math|Rotator|Lerp(Rotator) (Transformation|GetActorRotation) (Math|Rotator|FindLookatRotation (Variables|Default|GetPreviousLocation) (Transformation|GetActorLocation)) (Math|Curves|GetFloatValue (Variables|Default|GetVelocityRotationCurve) (Math|Vector|VectorLength (Transformation|GetComponentVelocity (Variables|Collision|GetCapsuleComponent)))) true) true)
  (Variables|Default|SetPreviousLocation (Transformation|GetActorLocation))
  (Variables|Default|SetPreviousRotation (Transformation|GetActorRotation)))

(fn HandleAerial
  (bind _capsulecomponent (Variables|Collision|GetCapsuleComponent))
  (if (Variables|Default|GetRightPressed)
    (Class|PrimitiveComponent|AddTorqueinDegrees (Variables|Collision|GetCapsuleComponent) (Math|Transform|TransformDirection (Transformation|GetRelativeTransform (Variables|Collision|GetCapsuleComponent)) "0.000000,0.000000,60000000.000000") "None" false))
  (if (Variables|Default|GetLeftPressed)
    (Class|PrimitiveComponent|AddTorqueinDegrees _capsulecomponent (Math|Transform|TransformDirection (Transformation|GetRelativeTransform _capsulecomponent) "0.000000,0.000000,-60000000.000000") "None" false)))